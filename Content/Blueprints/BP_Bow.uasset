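; BP_Bow is a bow whose string follows the player character's hand while aiming.
; It caches the third-person player character on BeginPlay and checks its IsAiming flag every Tick.
; While aiming, it moves the poseable mesh's string bone to the character's right-hand socket in world space; otherwise it resets that bone's transform.
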(event EventBeginPlay
  (bind _asbp_third_person_character (Utilities|Casting|CastToBP_ThirdPersonCharacter (Game|GetPlayerCharacter 0)))
  (Variables|Default|SetPlayerRef _asbp_third_person_character))

(event Collision|EventActorBeginOverlap
  (params (OtherActor :type Actor%20Object%20Reference)))

(event EventTick
  (params (DeltaSeconds :type Float%20%28single-precision%29))
  (if (Variables|/Script/PortfolioProject.PortfolioProjectCharacter|GetisAiming (Variables|Default|GetPlayerRef))
    (CallFunction|PullStringLogic)
    (else
      (CallFunction|ReleaseStringLogic))))

(fn ConstructionScript)

(fn PullStringLogic
  (Class|PoseableMeshComponent|SetBoneLocationbyName (Variables|Default|GetPoseableMesh1) "string" (Transformation|GetSocketLocation (Variables|/Script/Engine.Character|GetMesh (Variables|Default|GetPlayerRef)) "Hand_R") "WorldSpace"))

(fn ReleaseStringLogic
  (Class|PoseableMeshComponent|ResetBoneTransformbyName (Variables|Default|GetPoseableMesh1) "string"))